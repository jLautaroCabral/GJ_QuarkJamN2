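; Soccer ball the player aims, shoots with physics and steers sideways while it rolls.
; Before the shot, an arrow points at the target; ShootSoccerBall then applies an impulse toward it, scaled by shoot force, plus spin.
; Tick moves the camera boom with the ball, clamps sideways X speed to forward Y speed and stops the ball below a threshold.
; R resets the shot and hides the controller's force slider.
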(event `Key|R`
  (params (Key :type "Key Structure"))
  (bind _ballmesh (`self.BallMesh`))
  ;[1 1 1] Reset Shoot
  (:`Pressed`
    (if (`self.PlayerDidAShoot`)
      (`SceneComponent.K2_AttachToComponent` _ballmesh (`self.DefaultSceneRoot`) "None" "KeepRelative" "KeepRelative" "KeepRelative" true)
      (`SceneComponent.K2_SetRelativeLocation` _ballmesh (0.0 0.0 0.0) false false)
      (`SceneComponent.K2_SetRelativeRotation` :`self` _ballmesh)
      (`PrimitiveComponent.SetSimulatePhysics` _ballmesh false)
      (`self.UpdateCameraFollow`)
      (set `self.PlayerDidAShoot` false)
      (set `self.BallHasStoppedAfterShoot` false)
      (bind _asbp_player_controller (cast `/Game/Blueprints/BP_PlayerController` (`GameplayStatics.GetPlayerController` 0)))
      (`/Game/Blueprints/BP_PlayerController.ShowShootForceSlider` _asbp_player_controller false)
      (set `self.ShootDirectionAlreadyCalculated` false)
      (set `self.ShouldShowDirectionArrow` false))))

(event `EnhancedInput|/Game/Input/IA_Move`
  (params (ActionValue :type "Float (double-precision)") (ElapsedSeconds :type "Float (double-precision)") (TriggeredSeconds :type "Float (double-precision)") (InputAction :type "InputAction Object Reference" :default "/Game/Input/IA_Move.IA_Move"))
  ;[1 1 1] Ball Horizontal Input after player shoot
  (:`Triggered`
    (if (and (`self.PlayerDidAShoot`) (not (`self.BallHasStoppedAfterShoot`)))
      (`PrimitiveComponent.AddImpulse` (`self.BallMesh`) (`KismetMathLibrary.MakeVector` (* ActionValue (`self.HorizontalMovementSpeed`))) "None" false))))

(event `self.ReceiveTick`
  (params (DeltaSeconds :type "Float (single-precision)"))
  (bind (_ballcurrentvelocity_x _ballcurrentvelocity_y) (`KismetMathLibrary.BreakVector` (`self.BallCurrentVelocity`)))
  (bind _ballmesh (`self.BallMesh`))
  (bind (_ballcurrentvelocity_x_2 _ballcurrentvelocity_y_2 _ballcurrentvelocity_z) (`KismetMathLibrary.BreakVector` (`self.BallCurrentVelocity`)))
  (bind (_ballcurrentvelocity_x_3 _ballcurrentvelocity_y_3) (`KismetMathLibrary.BreakVector` (`self.BallCurrentVelocity`)))
  (bind _shootarrowdirection (`self.ShootArrowDirection`))
  (bind _directionarrowmesh (`self.DirectionArrowMesh`))
  (bind _returnvalue (`KismetMathLibrary.Abs` _ballcurrentvelocity_y_3))
  (if (`self.PlayerDidAShoot`)
    (`SceneComponent.SetHiddenInGame` (`self.DirectionArrowMesh`) true false)
    (bind _returnvalue_2 (`PrimitiveComponent.GetPhysicsLinearVelocity` (`self.BallMesh`) "None"))
    (set `self.BallCurrentVelocity` _returnvalue_2)
    (`self.UpdateCameraFollow`)
    (`PrimitiveComponent.SetPhysicsLinearVelocity` (`self.BallMesh`) (`KismetMathLibrary.MakeVector` (`KismetMathLibrary.FClamp` _ballcurrentvelocity_x_3 (* -1.0 _returnvalue) _returnvalue) _ballcurrentvelocity_y_2 _ballcurrentvelocity_z) false "None")
    (if (and (!= (`self.BallCurrentVelocity`) (`KismetMathLibrary.Vector_Zero`) :`ErrorTolerance` 1.0) (> (`self.StopBallThreshold`) (`KismetMathLibrary.Abs` _ballcurrentvelocity_y)))
      (`PrimitiveComponent.SetPhysicsLinearVelocity` _ballmesh (0.0 0.0 0.0) false "None")
      (`PrimitiveComponent.SetPhysicsAngularVelocityInDegrees` _ballmesh (0.0 0.0 0.0) false "None")
      (set `self.BallHasStoppedAfterShoot` true))
    (elif (not (`self.ShootDirectionAlreadyCalculated`))
      (if (`self.ShouldShowDirectionArrow`)
        (`SceneComponent.SetHiddenInGame` _directionarrowmesh false false)
        (`SceneComponent.K2_SetRelativeRotation` _directionarrowmesh (`KismetMathLibrary.FindRelativeLookAtRotation` (`SceneComponent.K2_GetComponentToWorld` (`self.BallMesh`)) _shootarrowdirection) false false)
        (`SceneComponent.SetWorldScale3D` _directionarrowmesh (`KismetMathLibrary.MakeVector` (`KismetMathLibrary.MultiplyMultiply_FloatFloat` (`KismetMathLibrary.VSize` (- _shootarrowdirection (`SceneComponent.K2_GetComponentLocation` (`self.BallMesh`)))) (/ 1.0 3.0)) 1.0 1.0))))))

(fn `ClampBallHorizontalVelocity`
  (bind (_ballcurrentvelocity_x _ballcurrentvelocity_y) (`KismetMathLibrary.BreakVector` (`self.BallCurrentVelocity`)))
  (bind (_ballcurrentvelocity_x_2 _ballcurrentvelocity_y_2 _ballcurrentvelocity_z) (`KismetMathLibrary.BreakVector` (`self.BallCurrentVelocity`)))
  (bind _returnvalue (`KismetMathLibrary.Abs` _ballcurrentvelocity_y))
  (`PrimitiveComponent.SetPhysicsLinearVelocity` (`self.BallMesh`) (`KismetMathLibrary.MakeVector` (`KismetMathLibrary.FClamp` _ballcurrentvelocity_x (* -1.0 _returnvalue) _returnvalue) _ballcurrentvelocity_y_2 _ballcurrentvelocity_z) false "None"))

(fn `ShootSoccerBall`
  (bind _ballmesh (`self.BallMesh`))
  (if (not (`self.PlayerDidAShoot`))
    (set `self.PlayerDidAShoot` true)
    (`SceneComponent.K2_AttachToComponent` _ballmesh (`self.DefaultSceneRoot`) "None" "SnapToTarget" "SnapToTarget" "SnapToTarget" true)
    (`SceneComponent.SetRelativeScale3D` _ballmesh (0.1 0.1 0.1))
    (`PrimitiveComponent.SetSimulatePhysics` _ballmesh true)
    (`PrimitiveComponent.AddImpulse` _ballmesh (* (- (`self.ShootArrowDirection`) (`SceneComponent.K2_GetComponentLocation` (`self.BallMesh`))) (`self.ShootForce`)) "None" false)
    (`PrimitiveComponent.SetPhysicsAngularVelocityInDegrees` _ballmesh (600.0 0.0 -600.0) false "None")
    (`KismetSystemLibrary.PrintString` (`KismetStringLibrary.Concat_StrStr` "Shoot force multiplier:  " (`KismetStringLibrary.Conv_DoubleToString` (`self.ShootForce`))) true true (struct :`G` 0.66 :`B` 1.0 :`A` 1.0) 4.0)))

(fn `UpdateCameraFollow`
  (`SceneComponent.K2_SetWorldLocation` (`self.CameraBoom`) (- (`SceneComponent.K2_GetComponentLocation` (`self.BallMesh`)) (0.0 10.0 0.0)) false false))

(fn `UserConstructionScript`)