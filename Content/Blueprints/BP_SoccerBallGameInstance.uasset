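; Game instance for the soccer ball game that owns the player's save slot, storing a high score and username.
; On Init it loads the existing BP_Save, or creates one with a zero score and a default username plus a random numeric suffix.
; Setter functions write to the save object and immediately save it to the slot; a getter returns the current high score.
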(event `self.ReceiveInit`
  (bind _returnvalue (`GameplayStatics.DoesSaveGameExist` (`self.PlayerGameSaveSlotName`)))
  (if _returnvalue
    (bind _returnvalue_2 (`GameplayStatics.LoadGameFromSlot` (`self.PlayerGameSaveSlotName`)))
    (set `self.PlayerGameSaveSlot` _returnvalue_2)
    (else
      (bind _returnvalue_3 (`GameplayStatics.CreateSaveGameObject` "/Game/Blueprints/BP_Save.BP_Save_C"))
      (set `self.PlayerGameSaveSlot` _returnvalue_3)
      (`self.Set And Save High Score` 0)
      (bind _usernamewithid (`self.Append New Generated ID` "DefaultUser"))
      (`self.Set And Save Username` _usernamewithid)
      (`self.Save Current Save Slot`))))

(fn `Append New Generated ID`
  (params (Username :type String))
  (returns (UsernameWithID :type String))
  (return (`KismetStringLibrary.Concat_StrStr` Username (`KismetStringLibrary.Concat_StrStr` "_" (`KismetStringLibrary.Conv_IntToString` (+ (* (`KismetMathLibrary.RandomInteger` 9) 1000) (* (`KismetMathLibrary.RandomInteger` 9) 100) (* (`KismetMathLibrary.RandomInteger` 9) 10) (* (`KismetMathLibrary.RandomInteger` 9) 1)))))))

(fn `Get Current High Score`
  (returns (`High Score` :type Integer))
  (bind _asbp_save (cast `/Game/Blueprints/BP_Save` (`self.PlayerGameSaveSlot`)))
  (return (`/Game/Blueprints/BP_Save.HighScore` _asbp_save)))

(fn `Save Current Save Slot`
  (`GameplayStatics.SaveGameToSlot` (`self.PlayerGameSaveSlot`) (`self.PlayerGameSaveSlotName`)))

(fn `Set And Save High Score`
  (params (HighScore :type Integer))
  (bind _asbp_save (cast `/Game/Blueprints/BP_Save` (`self.PlayerGameSaveSlot`)))
  (set `/Game/Blueprints/BP_Save.HighScore` HighScore _asbp_save)
  (`self.Save Current Save Slot`))

(fn `Set And Save Username`
  (params (PlayerUsername :type String))
  (bind _asbp_save (cast `/Game/Blueprints/BP_Save` (`self.PlayerGameSaveSlot`)))
  (set `/Game/Blueprints/BP_Save.PlayerUsername` PlayerUsername _asbp_save)
  (`self.Save Current Save Slot`))