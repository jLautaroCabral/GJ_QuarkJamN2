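; BP_Keeper is an AI-moved pawn that endlessly patrols an array of Destinations in order.
; BeginPlay and OnReset both start an AI MoveTo toward the actor at the current Target index, with a tight acceptance radius.
; Each successful arrival advances the index, wrapping to zero after the last entry, and issues the next move.
; Failed moves are unhandled, and OnReset resumes from the current index without clearing it.
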(event `self.K2_OnReset`
  (bind _returnvalue (+ (`self.Target`) 1))
  (`|AIMoveTo` self (0.0 0.0 0.0) (`|GetArrayItem` (`self.Destinations`) (`self.Target`)) 1.0 :!label _label
    (:`OnSuccess`
      (if (== _returnvalue (`KismetArrayLibrary.Array_Length` (`self.Destinations`)))
        (set `self.Target` 0)
        (goto _label)
        (else
          (set `self.Target` _returnvalue)
          (goto _label))))))

(event `self.ReceiveBeginPlay`
  (goto _label))

(fn `UserConstructionScript`)