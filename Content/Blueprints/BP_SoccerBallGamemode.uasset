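; Game mode for a soccer ball shooting game that owns the HUD and switches it between play and game over.
; On BeginPlay it creates the W_BallShootGameMode widget for player 0 and shows its top menu with the game-over overlay hidden.
; Game over focuses input on the UI and swaps the top menu for the overlay.
; Restarting the player returns input to game-only and prints a debug message.
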(event `self.ReceiveBeginPlay`
  (bind _gamemodeui (`self.GameModeUI`))
  (bind _returnvalue (`|CreateWidget` "/Game/UI/W_BallShootGameMode.W_BallShootGameMode_C" (`GameplayStatics.GetPlayerController` 0)))
  (bind _output_get (set `self.GameModeUI` _returnvalue))
  (`UserWidget.AddToViewport` _output_get 0)
  (`/Game/UI/W_BallShootGameMode.ShowGameOverOverlay` _gamemodeui false)
  (`/Game/UI/W_BallShootGameMode.ShowTopMenu` _gamemodeui true))

(event `OnGameOver`
  (bind _gamemodeui (`self.GameModeUI`))
  (`WidgetBlueprintLibrary.SetInputMode_UIOnlyEx` (`GameplayStatics.GetPlayerController` 0) _gamemodeui)
  (`/Game/UI/W_BallShootGameMode.ShowTopMenu` _gamemodeui false)
  (`/Game/UI/W_BallShootGameMode.ShowGameOverOverlay` _gamemodeui true))

(event `self.K2_OnRestartPlayer`
  (params (NewPlayer :type "Controller Object Reference"))
  (`KismetSystemLibrary.PrintString` "ON RESTART PLAYER" true true (struct :`R` 1.0 :`B` 0.031668 :`A` 1.0) 5.0)
  (`WidgetBlueprintLibrary.SetInputMode_GameOnly` (`GameplayStatics.GetPlayerController` 0)))

(fn `UserConstructionScript`)