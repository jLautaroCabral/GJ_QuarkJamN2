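; Player controller for a soccer ball game that lets the player aim and shoot the possessed BP_SoccerBall by touch or mouse.
; BeginPlay adds the Enhanced Input context and creates the W_Main widget with its force slider.
; Pressing traces under finger or cursor to set the ball's arrow direction; releasing locks it and shows the slider.
; FinalizeConfig&Shoot hides the slider and fires the ball after short delays.
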(event `self.ReceiveBeginPlay`
  (bind _returnvalue (subsystem `EnhancedInputLocalPlayerSubsystem`))
  ;[1 1 1] Input Mapping
  (set `self.bShowMouseCursor` true)
  (`/Engine/EditorBlueprintResources/StandardMacros.IsValid` _returnvalue
    (:`Is Valid`
      (`EnhancedInputSubsystemInterface.AddMappingContext` _returnvalue "/Game/Input/IMC_Default.IMC_Default" 0 (struct))
      (bind _returnvalue_2 (`|CreateWidget` "/Game/UI/W_Main.W_Main_C" self))
      (`UserWidget.AddToViewport` _returnvalue_2 0)
      (set `self.UI_Widget` _returnvalue_2)
      (set `self.Force Shoot Slider` (`/Game/UI/W_Main.ForceShootSlider` _returnvalue_2))
      (bind _asbp_soccer_ball (cast `/Game/Blueprints/BP_SoccerBall` (`GameplayStatics.GetPlayerPawn` 0)))
      (set `self.PlayerSoccerBall` _asbp_soccer_ball)
      (`self.ShowShootForceSlider` false))))

(event `EnhancedInput|/Game/Input/IA_Touch`
  (params (ActionValue :type Boolean) (ElapsedSeconds :type "Float (double-precision)") (TriggeredSeconds :type "Float (double-precision)") (InputAction :type "InputAction Object Reference" :default "/Game/Input/IA_Touch.IA_Touch"))
  (:`Triggered`
    (`self.Handle Draw Shoot DIrection Arrow Config` (`self.GetHitResultUnderFingerByChannel` "Touch1" "TraceTypeQuery1") :!label _label))
  (:`Started`
    (goto _label))
  (:`Completed`
    (goto _label :!via `On Release Input`)))

(event `EnhancedInput|/Game/Input/IA_Click`
  (params (ActionValue :type Boolean) (ElapsedSeconds :type "Float (double-precision)") (TriggeredSeconds :type "Float (double-precision)") (InputAction :type "InputAction Object Reference" :default "/Game/Input/IA_Click.IA_Click"))
  (:`Triggered`
    (`self.Handle Draw Shoot DIrection Arrow Config` (`self.GetHitResultUnderCursorByChannel` "TraceTypeQuery1") :!label _label_2))
  (:`Started`
    (goto _label_2))
  (:`Completed`
    (goto _label_2 :!via `On Release Input`)))

(event `Finalize Config & Shoot`
  ;[1 1 1] Finalize config and shoot the ball
  (`KismetSystemLibrary.Delay` 0.3)
  (`self.ShowShootForceSlider` false)
  (`KismetSystemLibrary.Delay` 0.2)
  (`/Game/Blueprints/BP_SoccerBall.ShootSoccerBall` (`self.PlayerSoccerBall`)))

(fn `ShowShootForceSlider`
  (params (Show :type Boolean))
  (bind _force_shoot_slider (`self.Force Shoot Slider`))
  (bind _minvalue (`Slider.MinValue` _force_shoot_slider))
  (if Show
    (`Widget.SetVisibility` _force_shoot_slider "Visible")
    (else
      (`Widget.SetVisibility` _force_shoot_slider "Hidden")))
  (`Slider.SetValue` _force_shoot_slider _minvalue)
  (set `/Game/UI/W_Main.PreviousValue` _minvalue (`self.UI_Widget`)))

(fn `UserConstructionScript`)