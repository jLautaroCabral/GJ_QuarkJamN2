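; Player controller that records the mouse path into a drawing widget while the left mouse button is held.
; On BeginPlay it creates and focuses W_Sample in Game and UI input mode with the cursor hidden.
; Each Tick during a press appends the DPI-scaled mouse position to the widget's Points array, skipping repeats of the last point.
; An empty array is never seeded here.
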(event `self.ReceiveBeginPlay`
  (bind _returnvalue (`|CreateWidget` "/Game/UI/W_Sample.W_Sample_C" self))
  (`UserWidget.AddToViewport` _returnvalue 0)
  (set `self.DrawingWidget` _returnvalue)
  (`WidgetBlueprintLibrary.SetInputMode_GameAndUIEx` null _returnvalue "DoNotLock" false)
  (set `self.bShowMouseCursor` false))

(event `self.ReceiveTick`
  (params (DeltaSeconds :type "Float (single-precision)"))
  (bind (_locationx _locationy) (`WidgetLayoutLibrary.GetMousePositionScaledByDPI` self))
  (bind (_locationx_2 _locationy_2) (`WidgetLayoutLibrary.GetMousePositionScaledByDPI` self))
  (bind _points (`/Game/UI/W_Sample.Points` (`self.DrawingWidget`)))
  (if (`self.IsLeftMouseButtonDown`)
    (if (> (`KismetArrayLibrary.Array_Length` (`/Game/UI/W_Sample.Points` (`self.DrawingWidget`))) 0)
      (if (not (== (`|GetArrayItem` _points (`KismetArrayLibrary.Array_LastIndex` _points)) (`KismetMathLibrary.MakeVector2D` _locationx_2 _locationy_2)))
        (`KismetArrayLibrary.Array_Add` (`/Game/UI/W_Sample.Points` (`self.DrawingWidget`)) (`KismetMathLibrary.MakeVector2D` _locationx _locationy))))))

(event `Key|LeftMouseButton`
  (params (Key :type "Key Structure"))
  (:`Pressed`
    (set `self.IsLeftMouseButtonDown` true))
  (:`Released`
    (set `self.IsLeftMouseButtonDown` false)))

(fn `UserConstructionScript`)